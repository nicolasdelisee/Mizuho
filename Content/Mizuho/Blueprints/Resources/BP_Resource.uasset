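; BP_Resource is a gatherable resource actor, apparently a tree given its depletion message.
; On BeginPlay it looks up ResourceRowName in DT_ResourceDataTable to set its static mesh and starting amount.
; GatherResource subtracts the requested amount, capped at what remains, from CurrentAmount.
; Depletion only prints a debug message; the actor is not destroyed.
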(event EventBeginPlay
  (bind _returnvalue (Utilities|GetDataTableRow "/Game/Mizuho/Data/Resources/DT_ResourceDataTable.DT_ResourceDataTable" (Variables|Default|GetResourceRowName))
    (:then
      (Components|StaticMesh|SetStaticMesh (Variables|Default|GetStaticMesh) (.Mesh (Utilities|Struct|BreakS_ResourceData _returnvalue)))
      (Variables|Default|SetCurrentAmount (.MaxAmount (Utilities|Struct|BreakS_ResourceData _returnvalue))))))

(event Collision|EventActorBeginOverlap
  (params (OtherActor :type Actor%20Object%20Reference)))

(event EventTick
  (params (DeltaSeconds :type Float%20%28single-precision%29)))

(fn ConstructionScript)

(fn GatherResource
  (params (AmountToGather :type Integer))
  (if (> (Variables|Default|GetCurrentAmount) (LocalVariables|GetGathered))
    (LocalVariables|SetGathered (Math|Integer|Min(Integer) AmountToGather (Variables|Default|GetCurrentAmount)))
    (Variables|Default|SetCurrentAmount (- (Variables|Default|GetCurrentAmount) (LocalVariables|GetGathered)))
    (if (<= (Variables|Default|GetCurrentAmount) 0)
      (Development|PrintString "Tree destroyed"))))