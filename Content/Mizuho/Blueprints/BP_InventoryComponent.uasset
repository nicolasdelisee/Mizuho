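; Inventory component that stores resource amounts by row name, with debug prints labeling its use for villager and building inventories.
; A single MaxCarryAmount caps the summed total of all resources in the map.
; AddResourceInInventory and AddResourceInStock share the same clamped-add logic, differing only in debug label, and return whatever amount did not fit.
; GetTotalInventory sums the map values and feeds both add functions and IsInventoryFull.
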(event EventBeginPlay)

(event EventTick
  (params (DeltaSeconds :type Float%20%28single-precision%29)))

(fn AddResourceinInventory
  (params (ResourceRowName :type Name) (Amount :type Integer))
  (bind _sum (CallFunction|GetTotalInventory))
  (Variables|Villager|SetCurrentCarrying _sum)
  (if (>= (Variables|Villager|GetCurrentCarrying) (Variables|Default|GetMaxCarryAmount))
    (Development|PrintString "Full inventory")
    ;[0.15 0.15 0.15 0.5] Older and simpler
    (return Amount)
    (else
      (LocalVariables|SetSpaceLeft (- (Variables|Default|GetMaxCarryAmount) (Variables|Villager|GetCurrentCarrying)))
      (LocalVariables|SetActualTaken (Math|Integer|Min(Integer) Amount (LocalVariables|GetSpaceLeft)))
      (LocalVariables|SetOldValue (.Value (Utilities|Map|Find (Variables|Default|GetResourceMap) ResourceRowName)))
      (LocalVariables|SetNewValue (+ (LocalVariables|GetOldValue) (LocalVariables|GetActualTaken)))
      (Utilities|Map|Add (Variables|Default|GetResourceMap) ResourceRowName (LocalVariables|GetNewValue))
      (bind _output_get (LocalVariables|SetRemainder (- Amount (LocalVariables|GetActualTaken))))
      (Development|PrintString (Utilities|String|Append "Villager inventory :" (Utilities|String|ToString(Integer) (LocalVariables|GetNewValue))))
      (return _output_get))))

(fn GetTotalInventory
  (Variables|Default|SetSum 0)
  (bind _keys (Utilities|Map|Keys (Variables|Default|GetResourceMap)))
  (for _array_element _keys
    (bind _output_get (LocalVariables|SetFoundValue (.Value (Utilities|Map|Find (Variables|Default|GetResourceMap) _array_element))))
    (Variables|Default|SetSum (+ _output_get (Variables|Default|GetSum))))
  (return (Variables|Default|GetSum)))

(fn IsInventoryFull
  (bind _sum (CallFunction|GetTotalInventory))
  (if (>= _sum (Variables|Default|GetMaxCarryAmount))
    (bind _output_get (Variables|Default|SetInventoryIsFull true))
    (return _output_get)
    (else
      (bind _output_get_2 (Variables|Default|SetInventoryIsFull false))
      (return _output_get_2))))

(fn AddResourceinStock
  (params (ResourceRowName :type Name) (Amount :type Integer))
  (bind _sum (CallFunction|GetTotalInventory))
  (Variables|Villager|SetCurrentCarrying _sum)
  (if (>= (Variables|Villager|GetCurrentCarrying) (Variables|Default|GetMaxCarryAmount))
    (Development|PrintString "Full inventory")
    ;[0.15 0.15 0.15 0.5] Older and simpler
    (return Amount)
    (else
      (LocalVariables|SetSpaceLeft (- (Variables|Default|GetMaxCarryAmount) (Variables|Villager|GetCurrentCarrying)))
      (LocalVariables|SetActualTaken (Math|Integer|Min(Integer) Amount (LocalVariables|GetSpaceLeft)))
      (LocalVariables|SetOldValue (.Value (Utilities|Map|Find (Variables|Default|GetResourceMap) ResourceRowName)))
      (LocalVariables|SetNewValue (+ (LocalVariables|GetOldValue) (LocalVariables|GetActualTaken)))
      (Utilities|Map|Add (Variables|Default|GetResourceMap) ResourceRowName (LocalVariables|GetNewValue))
      (bind _output_get (LocalVariables|SetRemainder (- Amount (LocalVariables|GetActualTaken))))
      (Development|PrintString (Utilities|String|Append "Building inventory :" (Utilities|String|ToString(Integer) (LocalVariables|GetNewValue))))
      (return _output_get))))