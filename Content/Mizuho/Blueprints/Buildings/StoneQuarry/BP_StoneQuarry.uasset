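; BP_StoneQuarry is the stone quarry building actor that opens a building popup when clicked.
; On BeginPlay it enables mouse click events and loads its default data from the StoneQuarry row of DT_BuildingDataTable.
; A click on its Box refreshes BuildingData from BP_GameInstance by BuildingId, then passes it and itself to the UIManager actor's popup toggle.
; An unconnected debug print of stored building data remains in the graph.
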(event OnClicked(Box)
  (params (TouchedComponent :type Primitive%20Component%20Object%20Reference) (ButtonPressed :type Key%20Structure))
  (bind _asbp_game_instance (Utilities|Casting|CastToBP_GameInstance (Game|GetGameInstance)))
  (bind _buildingdata (Default|GetBuildingbyId _asbp_game_instance (Variables|Default|GetBuildingId)))
  (Variables|Default|SetBuildingData _buildingdata)
  (bind _returnvalue (Actor|GetActorOfClass "/Game/Mizuho/UI/UIManager.UIManager_C"))
  (Default|ToggleBuildingPopup _returnvalue (Variables|Default|GetBuildingData) self))

(event EventBeginPlay
  (Variables|/Script/Engine.PlayerController|SetbEnableClickEvents (Game|GetPlayerController 0) true)
  (bind _returnvalue (Utilities|GetDataTableRow "/Game/Mizuho/Data/Buildings/DT_BuildingDataTable.DT_BuildingDataTable" "StoneQuarry")
    (:then
      (Variables|Default|SetBuildingData _returnvalue))))

(fn ConstructionScript)