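; Woodcutter camp building that tracks nearby resources and stores wood deposited by villagers.
; On BeginPlay it loads its building data table row and enables click events; clicking its box refreshes data from the game instance and toggles the UI manager's building popup.
; A work range sphere maintains the NearbyTrees list through overlaps.
; A setter stores the selected resource, and deposits pass only villager Wood quantities to the camp inventory.
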(event OnComponentBeginOverlap(WorkRangeSphere)
  (params (OverlappedComponent :type Primitive%20Component%20Object%20Reference) (OtherActor :type Actor%20Object%20Reference) (OtherComp :type Primitive%20Component%20Object%20Reference) (OtherBodyIndex :type Integer) (bFromSweep :type Boolean) (SweepResult :type Hit%20Result%20Structure%20%28by%20ref%29))
  (bind _asbp_resource (Utilities|Casting|CastToBP_Resource OtherActor))
  (Utilities|Array|Add (Variables|Default|GetNearbyTrees) _asbp_resource)
  (Variables|Default|SetBuildingActor self))

(event OnComponentEndOverlap(WorkRangeSphere)
  (params (OverlappedComponent :type Primitive%20Component%20Object%20Reference) (OtherActor :type Actor%20Object%20Reference) (OtherComp :type Primitive%20Component%20Object%20Reference) (OtherBodyIndex :type Integer))
  (bind _asbp_resource (Utilities|Casting|CastToBP_Resource OtherActor))
  (Utilities|Array|RemoveItem (Variables|Default|GetNearbyTrees) _asbp_resource))

(event OnClicked(Box)
  (params (TouchedComponent :type Primitive%20Component%20Object%20Reference) (ButtonPressed :type Key%20Structure :default "None"))
  (bind _asbp_game_instance (Utilities|Casting|CastToBP_GameInstance (Game|GetGameInstance)))
  (bind _buildingdata (Default|GetBuildingbyId _asbp_game_instance (Variables|Default|GetBuildingId)))
  (Variables|Default|SetBuildingData _buildingdata)
  (bind _returnvalue (Actor|GetActorOfClass "/Game/Mizuho/UI/UIManager.UIManager_C"))
  (Default|ToggleBuildingPopup _returnvalue (Variables|Default|GetBuildingData) self))

(event Custom|SetSelectedResource
  (params (NewResource :type E_ResourceType%20Enum :default "NewEnumerator3"))
  (Variables|Default|SetSelectedResource NewResource))

(event EventBeginPlay
  (Variables|/Script/Engine.PlayerController|SetbEnableClickEvents (Game|GetPlayerController 0) true)
  (bind _returnvalue (Utilities|GetDataTableRow "/Game/Mizuho/Data/Buildings/DT_BuildingDataTable.DT_BuildingDataTable" "WoodcutterCamp")
    (:then
      (Variables|Default|SetBuildingData _returnvalue))))

(fn ConstructionScript)

(fn DepositResourcesfromVillager
  (params (VillagerInventory :type BP%20Inventory%20Component%20Object%20Reference))
  (bind _keys (Utilities|Map|Keys (Variables|/Game/Mizuho/Blueprints/BP_InventoryComponent.BP_InventoryComponent_C|GetResourceMap VillagerInventory)))
  (for _array_element _keys
    (if (== _array_element "Wood")
      (bind _output_get (LocalVariables|SetQuantity (.Value (Utilities|Map|Find (Variables|/Game/Mizuho/Blueprints/BP_InventoryComponent.BP_InventoryComponent_C|GetResourceMap VillagerInventory) _array_element))))
      (Default|AddResourceinStock (Variables|Default|GetWoodcutterCampInventory) "None" _output_get))))