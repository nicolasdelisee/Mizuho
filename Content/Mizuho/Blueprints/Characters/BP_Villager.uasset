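; Villager character that wanders randomly when unemployed, toggles an info popup on click, and works as a woodcutter when assigned that job.
; Job changes resolve the building through the game instance, then AI MoveTo walks it to the camp and closest tree.
; A looping timer, timed from the resource DataTable, fills the inventory, pausing while the villager deposits at camp.
; Tree search toggles the camp between Wood and Bamboo when no trees are nearby.
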(event OnClicked(CapsuleComponent)
  (params (TouchedComponent :type Primitive%20Component%20Object%20Reference) (ButtonPressed :type Key%20Structure :default "None"))
  ;[0.15 0.15 0.15 0.5 32] Toggling Villager Popup
  (Utilities|Casting|CastToBP_GameInstance (Game|GetGameInstance))
  (bind _returnvalue (Actor|GetActorOfClass "/Game/Mizuho/UI/UIManager.UIManager_C"))
  (Default|ToggleVillagerPopup _returnvalue (Variables|Data|GetVillagerData) self))

(event Custom|Random%20Roam
  ;[0.15 0.15 0.15 0.5] Random Roam
  (AI|AIMoveTo self (.RandomLocation (AI|Navigation|GetRandomReachablePointinRadius (Transformation|GetActorLocation) (Variables|Movement|GetWanderRadius) 0 0)) 0 5.0 false
    (:OnSuccess
      (CallFunction|RandomRoam))))

(event Custom|OnJobChanged
  (bind _villagerdata (Variables|Data|GetVillagerData))
  (bind (_currenttask _profession) (Utilities|Struct|BreakS_VillagerData _villagerdata))
  (Variables|Data|SetProfession _profession)
  (Default|CallOnJobChangedUpdatePopup (|GenerictoText _profession) (|GenerictoText _currenttask))
  (Variables|Data|SetBuilding%20Id (Utilities|Struct|BreakS_VillagerData (Variables|Data|GetVillagerData)))
  (bind _asbp_game_instance (Utilities|Casting|CastToBP_GameInstance (Game|GetGameInstance)))
  (bind _buildingdata (Default|GetBuildingbyId _asbp_game_instance (Variables|Data|GetBuilding%20Id)))
  (Variables|Default|SetResourceProduced (.ResourceProduced (Utilities|Struct|BreakS_BuildingData _buildingdata)))
  (Variables|Default|SetBuildingLocation (.Location (Utilities|Struct|BreakS_BuildingData _buildingdata)))
  (switch Utilities|FlowControl|Switch|SwitchonE_VillagerProfession (Variables|Data|GetProfession)
    (:NewEnumerator2
      ;[0.15 0.05773 0.02294 0.5 32] Woodcutting
      (AI|AIMoveTo self (Variables|Default|GetBuildingLocation) 0 2e+02 false
        (:OnSuccess
          (bind _woodcuttercampactor (CallFunction|GetWoodcutterCampActor (Variables|Data|GetBuilding%20Id)))
          (Variables|Default|SetWoodcutterCampActor _woodcuttercampactor)
          (bind _closesttree (CallFunction|GetClosestTree))
          (Variables|Default|SetCurrentTree _closesttree)
          (if (Utilities|IsValid (Variables|Default|GetCurrentTree))
            (AI|AIMoveTo self (Transformation|GetActorLocation (Variables|Default|GetCurrentTree)) 0 1e+02 false
              (:OnSuccess
                (CallFunction|StartChoppingwithTimer)))
            (else
              (Development|PrintString "There is no tree close to the woodcutter camp."))))))))

(event Custom|StartChoppingWithTimer
  (params (TargetTree :type BP%20Resource%20Object%20Reference))
  ;[0.15 0.05773 0.02294 0.5 32] Woodcutting
  ;;[0.15 0.15 0.15 0.5] Chopping Tree
  (bind _returnvalue (Utilities|GetDataTableRow "/Game/Mizuho/Data/Resources/DT_ResourceDataTable.DT_ResourceDataTable" "Wood")
    (:then
      (bind _returnvalue_2 (Utilities|Time|SetTimerbyFunctionName 0 "ChopTree" (Utilities|Struct|BreakS_ResourceData _returnvalue) true false 2.0))
      (Variables|Default|SetChopTimerHandle _returnvalue_2))))

(event Custom|ChopTree
  (if (Utilities|IsValid (Variables|Default|GetCurrentTree))
    ;[0.15 0.05773 0.02294 0.5 32] Woodcutting
    (Variables|Default|SetRessourceToChop (Variables|/Game/Mizuho/Blueprints/Resources/BP_Resource.BP_Resource_C|GetResourceRowName (Variables|Default|GetCurrentTree)))
    ;;[0.15 0.15 0.15 0.5] Chopping Tree
    (bind _actualgathered (Default|GatherResource (Variables|Default|GetCurrentTree) 2))
    (Variables|Default|SetCutAmount _actualgathered)
    (Default|AddResourceinVillagerInventory (Variables|Default|GetVillagerInventory) (Variables|Default|GetRessourceToChop) (Variables|Default|GetCutAmount))
    ;;[0.15 0.15 0.15 0.5] Full Inventory
    (bind _inventoryisfull (Default|IsInventoryFull (Variables|Default|GetVillagerInventory)))
    (Variables|Default|SetInventory%20Is%20Full _inventoryisfull)
    (if (Variables|Default|GetInventory%20Is%20Full)
      (Utilities|Time|PauseTimerbyHandle (Variables|Default|GetChopTimerHandle))
      (AI|AIMoveTo self (Variables|Default|GetBuildingLocation) 0 5e+02 false
        (:OnSuccess
          (Default|DepositResourcesfromVillager (Variables|Default|GetWoodcutterCampActor) (Variables|Default|GetVillagerInventory))
          (CallFunction|DepositRessources)
          (Utilities|FlowControl|Delay 2.0)
          (bind _closesttree (CallFunction|GetClosestTree))
          (Variables|Default|SetCurrentTree _closesttree)
          (if (Utilities|IsValid (Variables|Default|GetCurrentTree))
            (AI|AIMoveTo self (Transformation|GetActorLocation (Variables|Default|GetCurrentTree)) 0 1e+02 false
              (:OnSuccess
                (Utilities|FlowControl|Delay 2.0)
                (Utilities|Time|UnpauseTimerbyHandle (Variables|Default|GetChopTimerHandle))))
            (else
              (Development|PrintString "There is no tree close to the woodcutter camp.")
              (CallFunction|StopChopping))))))))

(event Custom|StopChopping
  ;[0.15 0.05773 0.02294 0.5 32] Woodcutting
  (Utilities|Time|ClearTimerbyFunctionName 0 "ChopTimerHandle")
  (Variables|Default|SetCurrentTree 0))

(event Custom|DepositRessources
  (Utilities|Map|Clear (Variables|/Game/Mizuho/Blueprints/BP_InventoryComponent.BP_InventoryComponent_C|GetResourceMap (Variables|Default|GetVillagerInventory))))

(event EventBeginPlay
  (Variables|/Script/Engine.PlayerController|SetbEnableClickEvents (Game|GetPlayerController 0) true)
  (Variables|Data|SetProfession (Utilities|Struct|BreakS_VillagerData (Variables|Data|GetVillagerData)))
  (if (Utilities|Enum|Equal(Enum) (Variables|Data|GetProfession) "NewEnumerator0")
    ;[0.15 0.15 0.15 0.5] Idle Behavior
    (if (not (Utilities|Struct|BreakS_VillagerData (Variables|Data|GetVillagerData)))
      (CallFunction|RandomRoam))))

(fn ConstructionScript)

(fn SetVillagerDatainGame
  (params (VillagerData :type S%20Villager%20Data%20Structure))
  (Variables|Data|SetVillagerData VillagerData))

(fn SetGenderMesh
  (switch Utilities|FlowControl|Switch|SwitchonE_VillagerGender (Utilities|Struct|BreakS_VillagerData (Variables|Data|GetVillagerData))
    (:NewEnumerator0
      (Variables|/Script/Engine.SkeletalMeshComponent|SetSkeletalMeshAsset (Variables|Character|GetMesh) "/Game/Mizuho/Assets/Characters/Female/Villager_Female.Villager_Female"))
    (:NewEnumerator1
      (Variables|/Script/Engine.SkeletalMeshComponent|SetSkeletalMeshAsset (Variables|Character|GetMesh) "/Game/Mizuho/Assets/Characters/Male/Villager_Male.Villager_Male"))))

(fn GetClosestTree
  (if (== (Utilities|Array|Length (Variables|/Game/Mizuho/Blueprints/Buildings/WoodcutterCamp/BP_WoodcutterCamp.BP_WoodcutterCamp_C|GetNearbyTrees (Variables|Default|GetWoodcutterCampActor))) 0)
    (switch Utilities|FlowControl|Switch|SwitchonE_ResourceType (Variables|/Game/Mizuho/Blueprints/Buildings/WoodcutterCamp/BP_WoodcutterCamp.BP_WoodcutterCamp_C|GetSelectedResource (Variables|Default|GetWoodcutterCampActor))
      (:NewEnumerator0
        (Default|SetSelectedResource (Variables|Default|GetWoodcutterCampActor) "NewEnumerator7"))
      (:NewEnumerator7
        (Default|SetSelectedResource (Variables|Default|GetWoodcutterCampActor) "NewEnumerator0"))))
  (for _array_element (Variables|/Game/Mizuho/Blueprints/Buildings/WoodcutterCamp/BP_WoodcutterCamp.BP_WoodcutterCamp_C|GetNearbyTrees (Variables|Default|GetWoodcutterCampActor))
    (if (< (Math|Vector|VectorLength (- (Transformation|GetActorLocation _array_element) (Transformation|GetActorLocation self))) (LocalVariables|GetShortestDistance))
      (LocalVariables|SetShortestDistance (Math|Vector|VectorLength (- (Transformation|GetActorLocation _array_element) (Transformation|GetActorLocation self))))
      (LocalVariables|SetBestTree _array_element)))
  (return (LocalVariables|GetBestTree)))

(fn GetWoodcutterCampActor
  (params (BuildingId :type Integer))
  (bind _outactors (Actor|GetAllActorsOfClass "/Game/Mizuho/Blueprints/Buildings/WoodcutterCamp/BP_WoodcutterCamp.BP_WoodcutterCamp_C"))
  (for _array_element _outactors
    (if (== BuildingId (Variables|/Game/Mizuho/Blueprints/Buildings/WoodcutterCamp/BP_WoodcutterCamp.BP_WoodcutterCamp_C|GetBuildingId _array_element))
      (return _array_element))))

(fn GetClosestTrees
  (params (WantedResource :type E_ResourceType%20Enum :default "NewEnumerator3"))
  (bind _outactors (Actor|GetAllActorsOfClass "/Game/Mizuho/Blueprints/Buildings/WoodcutterCamp/BP_WoodcutterCamp.BP_WoodcutterCamp_C"))
  (for _array_element _outactors
    (if (== (Variables|Data|GetBuilding%20Id) (Variables|/Game/Mizuho/Blueprints/Buildings/WoodcutterCamp/BP_WoodcutterCamp.BP_WoodcutterCamp_C|GetBuildingId _array_element))
      (for _array_element_2 (Variables|/Game/Mizuho/Blueprints/Buildings/WoodcutterCamp/BP_WoodcutterCamp.BP_WoodcutterCamp_C|GetNearbyTrees _array_element)
        (if (< (Math|Vector|VectorLength (- (Transformation|GetActorLocation _array_element_2) (Transformation|GetActorLocation self))) (LocalVariables|GetShortestDistance))
          (LocalVariables|SetShortestDistance (Math|Vector|VectorLength (- (Transformation|GetActorLocation _array_element_2) (Transformation|GetActorLocation self))))
          (LocalVariables|SetBestTree _array_element_2)))
      (return (LocalVariables|GetBestTree)))))